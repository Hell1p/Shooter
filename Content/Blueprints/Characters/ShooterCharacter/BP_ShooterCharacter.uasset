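; Shooter character Blueprint that computes procedural weapon sway every Tick from view pitch and camera movement.
; Control pitch relative to the actor sets a position offset and slides the WeaponSwayScene component along X.
; Clamped frame-to-frame camera rotation deltas feed a smoothed rotation rate, which maps to a camera offset.
; Interp speed divides by delta time, so smoothing steps a fixed fraction per frame, smaller while aiming.
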(event `self.ReceiveTick`
  (params (DeltaSeconds :type "Float (single-precision)"))
  (`self.WeaponSway` (`self.CurrentCamRotation`) (select `bool` (`self.bAiming`) :`false` 10.0 :`true` 40.0)))

(fn `UserConstructionScript`)

(fn `WeaponSway`
  (params (CamRotPrev :type "Rotator Structure") (InterpSpeed :type "Float (double-precision)"))
  (locals (NewLocalVar :type "Float (double-precision)"))
  (bind _returnvalue (`GameplayStatics.GetWorldDeltaSeconds`))
  (bind (_camrotationrate_roll _camrotationrate_pitch _camrotationrate_yaw) (`KismetMathLibrary.BreakRotator` (`self.CamRotationRate`)))
  (bind (_returnvalue_roll _returnvalue_pitch) (`KismetMathLibrary.BreakRotator` (`KismetMathLibrary.NormalizedDeltaRotator` (`self.GetControlRotation`) (`self.K2_GetActorRotation`))))
  (bind (_relativelocation_x _relativelocation_y _relativelocation_z) (`KismetMathLibrary.BreakVector` (`SceneComponent.RelativeLocation` (`self.WeaponSwayScene`))))
  (bind _returnvalue_2 (`KismetMathLibrary.NormalizeToRange` _returnvalue_pitch -200.0 90.0))
  ;[1 1 1] Set socket location
  (`|ExecutionSequence`
    (:`then_0`
      (set `self.PitchOffsetPosition` (`KismetMathLibrary.MakeVector` 0.0 (`KismetMathLibrary.Lerp` 3.0 -3.0 _returnvalue_2) (`KismetMathLibrary.Lerp` 2.0 -2.0 _returnvalue_2)))
      (`SceneComponent.K2_SetRelativeLocation` (`self.WeaponSwayScene`) (`KismetMathLibrary.MakeVector` (`KismetMathLibrary.Lerp` 35.0 0.0 (`KismetMathLibrary.FClamp` (`KismetMathLibrary.NormalizeToRange` _returnvalue_2 0.0 0.5))) _relativelocation_y _relativelocation_z) false false))
    (:`then_1`
      ;[1 1 1] Set sway rotation
      (bind _output_get (set `self.CurrentCamRotation` (`SceneComponent.K2_GetComponentRotation` (`self.FollowCamera`))))
      (set `self.CamRotationRate` (`KismetMathLibrary.RInterpTo` (`self.CamRotationRate`) (`KismetMathLibrary.MakeRotator` (`KismetMathLibrary.FClamp` (* (.pitch (`KismetMathLibrary.NormalizedDeltaRotator` _output_get (`local.CamRotPrev`))) -1.0) -5.0 5.0) 0.0 (`KismetMathLibrary.FClamp` (.yaw (`KismetMathLibrary.NormalizedDeltaRotator` _output_get (`local.CamRotPrev`))) -5.0 5.0)) _returnvalue (/ (/ 1.0 _returnvalue) (`local.InterpSpeed`)))))
    (:`then_2`
      ;[1 1 1] Set camera offset
      (set `self.CamRotationOffset` (`KismetMathLibrary.MakeVector` (`KismetMathLibrary.Lerp` -6.0 6.0 (`KismetMathLibrary.NormalizeToRange` _camrotationrate_yaw -5.0 5.0)) 0.0 (`KismetMathLibrary.Lerp` -10.0 10.0 (`KismetMathLibrary.NormalizeToRange` _camrotationrate_roll -5.0 5.0)))))))